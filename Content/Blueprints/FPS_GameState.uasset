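; GameState Blueprint that tracks round progression and zombie counts for a round-based zombie FPS.
; BeginPlay caches the FPS game mode and the first player's character.
; IncreaseRound advances the round, scales the spawn count linearly within a clamped range, and pushes both to the player's HUD round widget.
; CheckIfRoundIsOver asks the game mode to start a new round once the zombie count reaches zero.
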(event `self.ReceiveBeginPlay`
  (bind _asfps_game_mode (cast `/Game/Blueprints/FPS_GameMode` (`GameplayStatics.GetGameMode`)))
  (set `self.GameModeRef` _asfps_game_mode)
  (bind _asfps_character (cast `/Game/Blueprints/FPS_Character` (`GameplayStatics.GetPlayerPawn` 0)))
  (set `self.PlayerRef` _asfps_character))

(fn `CheckIfRoundIsOver`
  (if (<= (`self.NumberOfZombies`) 0)
    (`/Game/Blueprints/FPS_GameMode.StartNewRound` (`self.GameModeRef`))))

(fn `IncreaseRound`
  (`/Engine/EditorBlueprintResources/StandardMacros.IncrementInt` (`self.CurrentRound`)
    (:`  `
      (bind _output_get (set `self.NumberOfZombiesToSpawn` (`KismetMathLibrary.Clamp` (`KismetMathLibrary.Round` (+ (* (`self.CurrentRound`) 1.5) 3.0)) 0 150)))
      (`/Game/Blueprints/UMG/UI_RoundNumberr.UpdateData` (`/Game/Blueprints/UMG/MainHUD.UI_RoundNumberr` (`/Game/Blueprints/FPS_Character.MainHUDRef` (`self.PlayerRef`))) (`self.CurrentRound`) _output_get))))

(fn `UserConstructionScript`)