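; AI controller that starts the enemy behavior tree on BeginPlay and turns perception updates into blackboard values.
; AISense identifies each sense by its index in the last sensed stimuli, so it depends on sense order.
; The first sets canSeePlayer; the second, for tagged noises, sets TargetLocation to the stimulus location and changes AI State.
; The third, damage, targets the player character's current location and switches AI State to chasing.
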(event `self.ReceiveBeginPlay`
  (`self.RunBehaviorTree` "/Game/Blueprints/AI/AI_BehaviorTree.AI_BehaviorTree")
  (bind _asai_character (cast `/Game/Blueprints/AI/AI_Character` (`self.K2_GetPawn`)))
  (set `self.AI_Character_Ref` _asai_character))

(event `self.AIPerception.OnPerceptionUpdated`
  (params (UpdatedActors :type "Array of Actor Object Reference (by ref)"))
  (for _array_element UpdatedActors
    (bind _info (`AIPerceptionComponent.GetActorsPerception` (`self.AIPerception`) _array_element))
    (`self.AI_Sense` (`.LastSensedStimuli` (break `ActorPerceptionBlueprintInfo` _info)))))

(fn `AI_Sense`
  (params (`AI Stimulis` :type "Array of AIStimulus Structure"))
  (locals (CurrentSense :type "AIStimulus Structure"))
  (bind _returnvalue (`AIBlueprintHelperLibrary.GetBlackboard` null))
  (bind _returnvalue_2 (`AIBlueprintHelperLibrary.GetBlackboard` null))
  (bind (_age _expirationage _strength _stimuluslocation _receiverlocation _tag _bsuccessfullysensed) (break `AIStimulus` (`local.CurrentSense`)))
  (for (_array_element _array_index) `AI Stimulis`
    (set `local.CurrentSense` _array_element)
    (switch `int` _array_index
      (:`0`
        (`BlackboardComponent.SetValueAsBool` (`AIBlueprintHelperLibrary.GetBlackboard` null) "canSeePlayer" (`.bSuccessfullySensed` (break `AIStimulus` (`local.CurrentSense`)))))
      (:`1`
        (if (== _tag "AI_Noice")
          (if _bsuccessfullysensed
            (`BlackboardComponent.SetValueAsVector` _returnvalue_2 "TargetLocation" _stimuluslocation)
            (`BlackboardComponent.SetValueAsEnum` _returnvalue_2 "AI State" 1))))
      (:`2`
        (if (`.bSuccessfullySensed` (break `AIStimulus` (`local.CurrentSense`)))
          (`KismetSystemLibrary.PrintString` "damage successfully sensed")
          (`BlackboardComponent.SetValueAsVector` _returnvalue "TargetLocation" (`self.K2_GetActorLocation` (`GameplayStatics.GetPlayerCharacter` 0)))
          (`BlackboardComponent.SetValueAsEnum` _returnvalue "AI State" 1)
          (`KismetSystemLibrary.PrintString` "set ui state to is chesing"))))))

(fn `UserConstructionScript`)