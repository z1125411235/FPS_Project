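; AI enemy character with a zombie melee montage that takes point and radius damage from the player until it dies.
; Point damage scales by critical modifier and the hit physical material's DestructibleDamageThresholdScale; radius damage falls off linearly with distance.
; Each hit reports to AI damage sense, updates health, and shows floating damage and hitmarker widgets.
; Death sets the blackboard flag, ragdolls the mesh with a weapon-based impulse, and destroys the capsule.
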(event `self.ReceiveBeginPlay`
  (bind _asfps_character (cast `/Game/Blueprints/FPS_Character` (`GameplayStatics.GetPlayerPawn` 0)))
  (set `self.PlayerRef` _asfps_character))

(event `/Game/Blueprints/Interfaces/TakeDamage.TakeDamage`
  (params (AmmoData :type "/Game/Blueprints/Structs/AmmoData Structure") (CriticalHitModiFier :type "Float (single-precision)") (HitResult :type "HitResult Structure"))
  (bind (_damage _criticalhitchance) (break `/Game/Blueprints/Structs/AmmoData` AmmoData))
  (bind (_bblockinghit _binitialoverlap _time _distance _location _impactpoint _normal _impactnormal _physmat _hitactor _hitcomponent _hitbonename) (`GameplayStatics.BreakHitResult` HitResult))
  (if (not (`self.isDead`))
    (bind _damagetoapply (`self.SetDamage` _damage _criticalhitchance CriticalHitModiFier HitResult))
    (`AISense_Damage.ReportDamageEvent` self (`GameplayStatics.GetPlayerCharacter` 0) _damagetoapply _impactpoint)
    (bind _isdead (`self.UpdateHealth` _damagetoapply))
    (bind _output_get (set `self.isDead` _isdead))
    (if _output_get
      (`self.Die` _impactpoint _hitbonename))
    (`self.FloatingDamage` _damagetoapply _impactpoint)
    (`/Engine/EditorBlueprintResources/StandardMacros.IsValid` (`self.HitmarkerRef`) :!label _label
      (:`Is Valid`
        (`Widget.RemoveFromParent` (`self.HitmarkerRef`)))
      (:`Is Not Valid`
        _))
    (bind _returnvalue (`|CreateWidget` "/Game/Blueprints/UMG/UI_Hitmarker.UI_Hitmarker_C" null (`self.isDead`)))
    (bind _output_get_2 (set `self.HitmarkerRef` _returnvalue))
    (`UserWidget.AddToViewport` _output_get_2 0)))

(event `/Game/Blueprints/Interfaces/TakeDamage.TakeRadiusDamage`
  (params (GroundHitResult :type "HitResult Structure") (AmmoData :type "/Game/Blueprints/Structs/AmmoData Structure") (CriticalHitDamageModlfier :type "Float (single-precision)"))
  (bind (_damage _criticalhitchance _damageradus) (break `/Game/Blueprints/Structs/AmmoData` AmmoData))
  (bind (_bblockinghit _binitialoverlap _time _distance _location _impactpoint _normal _impactnormal _physmat _hitactor _hitcomponent _hitbonename) (`GameplayStatics.BreakHitResult` GroundHitResult))
  (if (not (`self.isDead`))
    (bind _damagetoapply (`self.SetRadiusDamage` _damage 0.0 _damageradus _impactpoint))
    (`AISense_Damage.ReportDamageEvent` self (`GameplayStatics.GetPlayerCharacter` 0) _damagetoapply _impactpoint)
    (bind _isdead (`self.UpdateHealth` _damagetoapply))
    (bind _output_get (set `self.isDead` _isdead))
    (if _output_get
      (`self.Die` _impactpoint _hitbonename))
    (`self.FloatingDamage` _damagetoapply _impactpoint)
    (goto _label)))

(event `self.FloatingDamage`
  (params (Damage :type "Float (single-precision)") (ImpactPoint :type "Vector Structure"))
  (bind (_x _y) (`KismetMathLibrary.BreakVector2D` (`WidgetLayoutLibrary.ProjectWorldLocationToWidgetPosition` (`GameplayStatics.GetPlayerController` 0) ImpactPoint)))
  (bind _returnvalue (`|CreateWidget` "/Game/Blueprints/UMG/UI_FloatingDamage.UI_FloatingDamage_C" null Damage))
  (`Widget.SetRenderTranslation` (`/Game/Blueprints/UMG/UI_FloatingDamage.ScreenPositionSizeBox` _returnvalue) (`KismetMathLibrary.MakeVector2D` (+ (+ _x -50.0) (`KismetMathLibrary.RandomFloatInRange` -25.0 25.0)) (+ (+ _y -100.0) (`KismetMathLibrary.RandomFloatInRange` -10.0 10.0))))
  (`UserWidget.AddToViewport` _returnvalue 0))

(event `/Game/Blueprints/AI/Interfaces/MeleeAttack.Melee`
  (`|PlayMontage` (`self.Mesh`) "/Game/Blueprints/AI/Animations/Zombie_Attack_Montage.Zombie_Attack_Montage"))

(fn `Die`
  (params (ImpactPoint :type "Vector Structure") (BoneName :type Name))
  (bind _mesh (`self.Mesh`))
  (bind _playerref (`self.PlayerRef`))
  (`BlackboardComponent.SetValueAsBool` (`AIBlueprintHelperLibrary.GetBlackboard` (`self.GetController`)) "isDead" true)
  (`PrimitiveComponent.SetSimulatePhysics` _mesh true)
  (`PrimitiveComponent.AddImpulseAtLocation` _mesh (* (`KismetMathLibrary.GetDirectionUnitVector` (`self.K2_GetActorLocation` _playerref) (`self.K2_GetActorLocation`)) (select `/Game/Blueprints/Enums/HasWeapon` (`/Game/Blueprints/FPS_Character.HasWeaponEnum` _playerref) :`NewEnumerator0` 10000.0 :`NewEnumerator1` (`/Game/Blueprints/Weapons/BP_WeaponBase.KillImpulse` (`/Game/Blueprints/FPS_Character.CurrentWeapon` _playerref)))) ImpactPoint BoneName)
  (`ActorComponent.K2_DestroyComponent` (`self.CapsuleComponent`)))

(fn `SetDamage`
  (params (Damage :type "Float (double-precision)") (CriticalHitChance :type "Float (double-precision)") (CriticalDamageModifier :type "Float (double-precision)") (HitResult :type "HitResult Structure"))
  (returns (DamageToApply :type "Float (double-precision)") (`WasCritical?` :type Boolean))
  (locals (LocalDamageAmt :type "Float (double-precision)") (LocalIsCriticalHit :type Boolean))
  (set `local.LocalDamageAmt` Damage)
  (`|ExecutionSequence`
    (:`then_0`
      (bind _output_get (set `local.LocalIsCriticalHit` (< CriticalHitChance (`KismetMathLibrary.RandomFloatInRange` 0.0))))
      (if _output_get
        (set `local.LocalDamageAmt` (* (`local.LocalDamageAmt`) CriticalDamageModifier))))
    (:`then_1`
      (set `local.LocalDamageAmt` (* (`local.LocalDamageAmt`) (`PhysicalMaterial.DestructibleDamageThresholdScale` (`.PhysMat` (`GameplayStatics.BreakHitResult` HitResult))))))
    (:`then_2`
      (return (`local.LocalDamageAmt`) (`local.LocalIsCriticalHit`)))))

(fn `SetRadiusDamage`
  (params (Damage :type "Float (double-precision)") (CriticalHitChance :type "Float (double-precision)") (Radius :type "Float (double-precision)") (GroundPoint :type "Vector Structure"))
  (returns (DamageToApply :type "Float (double-precision)") (`WasCritical?` :type Boolean))
  (locals (LocalDamageAmt :type "Float (double-precision)") (LocalIsCriticalHit :type Boolean))
  (set `local.LocalDamageAmt` Damage)
  (`|ExecutionSequence`
    (:`then_0`
      (set `local.LocalIsCriticalHit` (< CriticalHitChance (`KismetMathLibrary.RandomFloatInRange` 0.0))))
    (:`then_1`
      (return (`KismetMathLibrary.FClamp` (* (- 1.0 (/ (`KismetMathLibrary.VSize` (- GroundPoint (`self.K2_GetActorLocation`))) Radius)) (`local.LocalDamageAmt`)) 0.0 Damage) (`local.LocalIsCriticalHit`)))))

(fn `UpdateHealth`
  (params (Damage :type "Float (double-precision)"))
  (returns (IsDead :type Boolean))
  (locals (LocalIsDead :type Boolean))
  (`|ExecutionSequence`
    (:`then_0`
      (if (>= Damage (`self.CurrentHealth`))
        (set `local.LocalIsDead` true)
        (set `self.CurrentHealth` 0.0)
        (else
          (set `self.CurrentHealth` (- (`self.CurrentHealth`) Damage)))))
    (:`then_1`
      (return (`local.LocalIsDead`)))))

(fn `UserConstructionScript`)